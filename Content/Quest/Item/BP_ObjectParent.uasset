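; Parent Blueprint for quest item objects that the top-down character picks up into the inventory.
; Clicking the SphereDetection component flags the item as Grabbable.
; When BP_TopDownCharacter begins overlapping SphereCollPP on a flagged item, the item adds itself to the Inventaire collection on BP_GameInstance, then destroys its actor.
; The pickup check runs only when an overlap begins, and the flag is never cleared here.
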(event `self.SphereDetection.OnClicked`
  (params (TouchedComponent :type "PrimitiveComponent Object Reference") (ButtonPressed :type "Key Structure"))
  (set `self.Grabbable?` true))

(event `self.SphereCollPP.OnComponentBeginOverlap`
  (params (OverlappedComponent :type "PrimitiveComponent Object Reference") (OtherActor :type "Actor Object Reference") (OtherComp :type "PrimitiveComponent Object Reference") (OtherBodyIndex :type Integer) (bFromSweep :type Boolean) (SweepResult :type "HitResult Structure (by ref)"))
  (cast `/Game/TopDown/Blueprints/BP_TopDownCharacter` OtherActor)
  (if (`self.Grabbable?`)
    (`BlueprintSetLibrary.Set_Add` (`/Game/TopDown/Blueprints/BP_GameInstance.Inventaire` (cast `/Game/TopDown/Blueprints/BP_GameInstance` (`GameplayStatics.GetGameInstance`) :!pure true)) self)
    (`self.K2_DestroyActor`)))

(fn `UserConstructionScript`)