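; Quest NPC that talks when the top-down character overlaps its sphere.
; On contact it can give its quest through BP_GameInstance, if set as a giver and that quest is not already active.
; It plays an alternate dialog and completes the last quest step when its first ChangeDialog key matches the active quest and the second-to-last step is done.
; Otherwise it plays the default dialog and completes the first step.
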(event `self.ReceiveBeginPlay`
  (bind _asbp_game_instance (cast `/Game/TopDown/Blueprints/BP_GameInstance` (`GameplayStatics.GetGameInstance`)))
  (set `self.GI` _asbp_game_instance))

(event `self.SpherePP.OnComponentBeginOverlap`
  (params (OverlappedComponent :type "PrimitiveComponent Object Reference") (OtherActor :type "Actor Object Reference") (OtherComp :type "PrimitiveComponent Object Reference") (OtherBodyIndex :type Integer) (bFromSweep :type Boolean) (SweepResult :type "HitResult Structure (by ref)"))
  (cast `/Game/TopDown/Blueprints/BP_TopDownCharacter` OtherActor)
  (`self.SpeakPP`))

(event `SpeakPP`
  (bind _checkquestactive (`/Game/TopDown/Blueprints/BP_GameInstance.CheckQuestActive` (`self.GI`)))
  (`|ExecutionSequence`
    (:`then_0`
      (if (and (`|EnumInequality` (`/Game/TopDown/Blueprints/BP_GameInstance.QuestActive` (`self.GI`)) (`/Game/Quest/QuestManager/BP_QuestManager.NameQuest` (`self.WhichQuest?`))) (`self.DonneQuete?`))
        (`/Game/TopDown/Blueprints/BP_GameInstance.New Quest` (`self.GI`) (`self.WhichQuest?`))))
    (:`then_1`
      (bind _keys (`BlueprintMapLibrary.Map_Keys` (`self.ChangeDialog`)))
      (if (and (`|EnumEquality` (`|GetArrayItem` _keys) (`/Game/TopDown/Blueprints/BP_GameInstance.QuestActive` (`self.GI`))) (`|GetArrayItem` _checkquestactive (- (`KismetArrayLibrary.Array_Length` _checkquestactive) 2)))
        (`self.BaseDialog` "NewEnumerator17")
        (`KismetArrayLibrary.Array_Set` (`/Game/TopDown/Blueprints/BP_GameInstance.CheckQuestActive` (`self.GI`)) (- (`KismetArrayLibrary.Array_Length` (`/Game/TopDown/Blueprints/BP_GameInstance.CheckQuestActive` (`self.GI`))) 1) true)
        (else
          (`self.BaseDialog` "NewEnumerator0")
          (`KismetArrayLibrary.Array_Set` (`/Game/TopDown/Blueprints/BP_GameInstance.CheckQuestActive` (`self.GI`)) 0 true))))))

(fn `UserConstructionScript`
  (`parent.UserConstructionScript`))