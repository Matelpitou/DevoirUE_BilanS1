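; BP_Totem is a quest totem where the player places a required inventory item, revealing a skeletal mesh hidden at BeginPlay.
; When BP_TopDownCharacter overlaps the box, it checks the GameInstance's active quest, step flag and held item against QuestActiveStep and ItemAPlacer.
; A match empties the inventory, marks the item placed, shows the mesh and sets that same step flag true.
; Each overlap also prints the three checks for debugging.
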(event `self.ReceiveBeginPlay`
  (`SceneComponent.SetHiddenInGame` (`self.SkeletalMesh`) true false)
  (bind _asbp_game_instance (cast `/Game/TopDown/Blueprints/BP_GameInstance` (`GameplayStatics.GetGameInstance`)))
  (set `self.GI` _asbp_game_instance))

(event `self.Box.OnComponentBeginOverlap`
  (params (OverlappedComponent :type "PrimitiveComponent Object Reference") (OtherActor :type "Actor Object Reference") (OtherComp :type "PrimitiveComponent Object Reference") (OtherBodyIndex :type Integer) (bFromSweep :type Boolean) (SweepResult :type "HitResult Structure (by ref)"))
  (bind _questactive_step (`self.QuestActive&Step`))
  (bind _returnvalue (== (`self.ItemAPlacer`) (`/Game/TopDown/Blueprints/BP_GameInstance.Inventaire` (`self.GI`))))
  (cast `/Game/TopDown/Blueprints/BP_TopDownCharacter` OtherActor)
  (bind _keys (`BlueprintMapLibrary.Map_Keys` _questactive_step))
  (bind _values (`BlueprintMapLibrary.Map_Values` _questactive_step))
  (`|ExecutionSequence`
    (:`then_0`
      (bind _returnvalue_2 (`|EnumEquality` (`|GetArrayItem` _keys) (`/Game/TopDown/Blueprints/BP_GameInstance.QuestActive` (`self.GI`))))
      (bind _output (`|GetArrayItem` (`/Game/TopDown/Blueprints/BP_GameInstance.CheckQuestActive` (`self.GI`)) (`|GetArrayItem` _values)))
      (if (and _returnvalue_2 _output _returnvalue)
        (set `self.ItemPlacer?` true)
        (set `/Game/TopDown/Blueprints/BP_GameInstance.Inventaire` null (`self.GI`))
        (`SceneComponent.SetHiddenInGame` (`self.SkeletalMesh`) false false)
        (bind _values_2 (`BlueprintMapLibrary.Map_Values` (`self.QuestActive&Step`)))
        (`KismetArrayLibrary.Array_Set` (`/Game/TopDown/Blueprints/BP_GameInstance.CheckQuestActive` (`self.GI`)) (`|GetArrayItem` _values_2) true)))
    (:`then_1`
      (`KismetSystemLibrary.PrintString` (`KismetStringLibrary.Conv_BoolToString` _returnvalue_2)))
    (:`then_2`
      (`KismetSystemLibrary.PrintString` (`KismetStringLibrary.Conv_BoolToString` _output)))
    (:`then_3`
      (`KismetSystemLibrary.PrintString` (`KismetStringLibrary.Conv_BoolToString` _returnvalue)))))

(fn `UserConstructionScript`)